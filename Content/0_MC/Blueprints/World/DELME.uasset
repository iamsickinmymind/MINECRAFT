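; Voxel terrain chunk actor that builds a block of noise-shaped cubes around its location, with identical generation in the Construction Script and BeginPlay.
; 2D simplex noise at world voxel coordinates offsets column heights, and 3D noise carves holes, using a separate fixed cutoff for the randomly jittered top layer.
; Remaining voxels become scaled instances in per-material Instanced Static Mesh components, chosen by snow and grass height thresholds.
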(event `self.ReceiveBeginPlay`
  (bind _bp_area_2n_1_ (`self.BP_Area(2n-1)`))
  (bind _bp_instances (`self.BP_Instances`))
  (bind _bp_depth_2n_1_ (`self.BP_Depth(2n-1)`))
  (bind _bp_voxelsize (`self.BP_VoxelSize`))
  (bind _bp_worldvoxelpos_z_noised (`self.BP_WorldVoxelPos_Z_Noised`))
  (bind (_returnvalue_x _returnvalue_y _returnvalue_z) (`KismetMathLibrary.BreakVector` (/ (`self.K2_GetActorLocation`) (`KismetMathLibrary.Conv_IntToDouble` (`self.BP_VoxelSize`)))))
  (`self.BP_Initialize`)
  ;[1 1 1] Loops
  (for _index (range (* _bp_area_2n_1_ -1) (+ _bp_area_2n_1_ 1))
    (set `self.BP_LocalVoxelPos_X` _index)
    (for _index_2 (range (* _bp_area_2n_1_ -1) (+ _bp_area_2n_1_ 1))
      (set `self.BP_LocalVoxelPos_Y` _index_2)
      (for _index_3 (range (* _bp_depth_2n_1_ -1) (+ _bp_depth_2n_1_ 1))
        (set `self.BP_LocalVoxelPos_Z` _index_3)
        ;[1 1 1] Base Voxel Calculation
        (set `self.BP_WorldVoxelPos_X` (+ (`self.BP_LocalVoxelPos_X`) (`KismetMathLibrary.FFloor` _returnvalue_x)))
        (set `self.BP_WorldVoxelPos_Y` (+ (`self.BP_LocalVoxelPos_Y`) (`KismetMathLibrary.FFloor` _returnvalue_y)))
        (set `self.BP_WorldVoxelPos_Z_PreNoise` (+ (`self.BP_LocalVoxelPos_Z`) (`KismetMathLibrary.FFloor` _returnvalue_z)))
        ;[1 1 1] Calculate 2D Noise
        (bind _returnvalue (`SimplexNoiseBPLibrary.SimplexNoise2D` (`KismetMathLibrary.Conv_IntToDouble` (* _bp_voxelsize (`self.BP_WorldVoxelPos_X`))) (`KismetMathLibrary.Conv_IntToDouble` (* _bp_voxelsize (`self.BP_WorldVoxelPos_Y`))) (`self.BP_Noise Density`)))
        (set `self.BP_WorldVoxelPos_Z_Noised` (* (- (`KismetMathLibrary.FFloor` (* (`self.BP_Noise Scale`) _returnvalue)) (`self.BP_LocalVoxelPos_Z`)) (`self.BP_VoxelSize`)))
        (if (< (* (`self.BP_LocalVoxelPos_Z`) -1) (- (`self.BP_Depth(2n-1)`) (`KismetMathLibrary.RandomIntegerInRange` 0 1)))
          ;[1 1 1] 3D Noise
          (bind _shouldcutoff_ (`self.BP_Get3DNoise` (`self.BP_3D CutOff Noise Treshold`) (`self.BP_3D Noise Density`)))
          (if (not _shouldcutoff_)
            ;[1 1 1] Spawn Cube Instance
            (if (> _bp_worldvoxelpos_z_noised (`self.BP_SnowTreshold`)) :!label _label
              (`self.BP_AddVoxelInstanceOfType` (`|GetArrayItem` _bp_instances))
              (elif (< _bp_worldvoxelpos_z_noised (`self.BP_GrassTreshold`))
                (`self.BP_AddVoxelInstanceOfType` (`|GetArrayItem` _bp_instances 1))
                (else
                  (`self.BP_AddVoxelInstanceOfType` (`|GetArrayItem` _bp_instances 2))))))
          (else
            (bind _shouldcutoff__2 (`self.BP_Get3DNoise` -0.5 0.025))
            (if (not _shouldcutoff__2)
              (goto _label))))))))

(fn `BP_AddVoxelInstanceOfType`
  (params (`Instanced Mesh Component` :type "InstancedStaticMeshComponent Object Reference"))
  (`InstancedStaticMeshComponent.AddInstance` `Instanced Mesh Component` (`KismetMathLibrary.MakeTransform` (`KismetMathLibrary.MakeVector` (`KismetMathLibrary.Conv_IntToDouble` (* (`self.BP_VoxelSize`) (`self.BP_LocalVoxelPos_X`))) (`KismetMathLibrary.Conv_IntToDouble` (* (`self.BP_VoxelSize`) (`self.BP_LocalVoxelPos_Y`))) (`KismetMathLibrary.Conv_IntToDouble` (`self.BP_WorldVoxelPos_Z_Noised`))) (struct) (* (1.0 1.0 1.0) (/ (`self.BP_VoxelSize`) 100)))))

(fn `BP_Get3DNoise`
  (params (`Noise Cutoff` :type "Float (double-precision)") (`Noise Density` :type "Float (double-precision)"))
  (returns (`ShouldCutoff?` :type Boolean))
  (bind _bp_voxelsize (`self.BP_VoxelSize`))
  (bind _returnvalue (`SimplexNoiseBPLibrary.SimplexNoise3D` (`KismetMathLibrary.Conv_IntToDouble` (* _bp_voxelsize (`self.BP_WorldVoxelPos_X`))) (`KismetMathLibrary.Conv_IntToDouble` (* _bp_voxelsize (`self.BP_WorldVoxelPos_Y`))) (`KismetMathLibrary.Conv_IntToDouble` (* (`self.BP_WorldVoxelPos_Z_Noised`) _bp_voxelsize)) `Noise Density`))
  (return (<= _returnvalue `Noise Cutoff`)))

(fn `BP_Initialize`
  (for _index (range (`BlueprintMapLibrary.Map_Length` (`self.BP_BlockMaterialTypes`)))
    (bind _returnvalue (`AddComponent|NODE_AddInstancedStaticMeshComponent-0`))
    (`KismetArrayLibrary.Array_Add` (`self.BP_Instances`) _returnvalue)
    (`StaticMeshComponent.SetStaticMesh` _returnvalue (`self.BP_StaticMesh`))
    (`PrimitiveComponent.SetMaterial` _returnvalue 0 (`BlueprintMapLibrary.Map_Find` (`self.BP_BlockMaterialTypes`) _index))))

(fn `UserConstructionScript`
  (bind _bp_area_2n_1_ (`self.BP_Area(2n-1)`))
  (bind _bp_instances (`self.BP_Instances`))
  (bind _bp_depth_2n_1_ (`self.BP_Depth(2n-1)`))
  (bind _bp_voxelsize (`self.BP_VoxelSize`))
  (bind _bp_worldvoxelpos_z_noised (`self.BP_WorldVoxelPos_Z_Noised`))
  (bind (_returnvalue_x _returnvalue_y _returnvalue_z) (`KismetMathLibrary.BreakVector` (/ (`self.K2_GetActorLocation`) (`KismetMathLibrary.Conv_IntToDouble` (`self.BP_VoxelSize`)))))
  (`self.BP_Initialize`)
  ;[1 1 1] Loops
  (for _index (range (* _bp_area_2n_1_ -1) (+ _bp_area_2n_1_ 1))
    (set `self.BP_LocalVoxelPos_X` _index)
    (for _index_2 (range (* _bp_area_2n_1_ -1) (+ _bp_area_2n_1_ 1))
      (set `self.BP_LocalVoxelPos_Y` _index_2)
      (for _index_3 (range (* _bp_depth_2n_1_ -1) (+ _bp_depth_2n_1_ 1))
        (set `self.BP_LocalVoxelPos_Z` _index_3)
        ;[1 1 1] Base Voxel Calculation
        (set `self.BP_WorldVoxelPos_X` (+ (`self.BP_LocalVoxelPos_X`) (`KismetMathLibrary.FFloor` _returnvalue_x)))
        (set `self.BP_WorldVoxelPos_Y` (+ (`self.BP_LocalVoxelPos_Y`) (`KismetMathLibrary.FFloor` _returnvalue_y)))
        (set `self.BP_WorldVoxelPos_Z_PreNoise` (+ (`self.BP_LocalVoxelPos_Z`) (`KismetMathLibrary.FFloor` _returnvalue_z)))
        ;[1 1 1] Calculate 2D Noise
        (bind _returnvalue (`SimplexNoiseBPLibrary.SimplexNoise2D` (`KismetMathLibrary.Conv_IntToDouble` (* _bp_voxelsize (`self.BP_WorldVoxelPos_X`))) (`KismetMathLibrary.Conv_IntToDouble` (* _bp_voxelsize (`self.BP_WorldVoxelPos_Y`))) (`self.BP_Noise Density`)))
        (set `self.BP_WorldVoxelPos_Z_Noised` (* (- (`KismetMathLibrary.FFloor` (* (`self.BP_Noise Scale`) _returnvalue)) (`self.BP_LocalVoxelPos_Z`)) (`self.BP_VoxelSize`)))
        (if (< (* (`self.BP_LocalVoxelPos_Z`) -1) (- (`self.BP_Depth(2n-1)`) (`KismetMathLibrary.RandomIntegerInRange` 0 1)))
          ;[1 1 1] 3D Noise
          (bind _shouldcutoff_ (`self.BP_Get3DNoise` (`self.BP_3D CutOff Noise Treshold`) (`self.BP_3D Noise Density`)))
          (if (not _shouldcutoff_)
            ;[1 1 1] Spawn Cube Instance
            (if (> _bp_worldvoxelpos_z_noised (`self.BP_SnowTreshold`)) :!label _label
              (`self.BP_AddVoxelInstanceOfType` (`|GetArrayItem` _bp_instances))
              (elif (< _bp_worldvoxelpos_z_noised (`self.BP_GrassTreshold`))
                (`self.BP_AddVoxelInstanceOfType` (`|GetArrayItem` _bp_instances 1))
                (else
                  (`self.BP_AddVoxelInstanceOfType` (`|GetArrayItem` _bp_instances 2))))))
          (else
            (bind _shouldcutoff__2 (`self.BP_Get3DNoise` -0.5 0.025))
            (if (not _shouldcutoff__2)
              (goto _label))))))))